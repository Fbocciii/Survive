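; BP_ContainerMaster is a master Blueprint for interactable inventory containers.
; On BeginPlay it copies its ItemsA array slot by slot into the Inventory of its BPInventoryComponent.
; Interact runs the parent implementation, then toggles the component's inventory only when the interactor casts to ThirdPersonCharacter.
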(event `self.ReceiveBeginPlay`
  (for (_array_element _array_index) (`self.ItemsA`)
    (`KismetArrayLibrary.Array_Set` (`InventoryComponent.Inventory` (`self.BP_InventoryComponent`)) _array_index _array_element)))

(fn `Interact`
  (params (Interactor :type "Actor Object Reference"))
  (returns (Success :type Boolean))
  (bind _success (`parent.Interact` Interactor))
  (cast `/Game/ThirdPersonCPP/Blueprints/ThirdPersonCharacter` Interactor)
  (`/Game/InventorySystem/BP_InventoryComponent.ToggleInventory` (`self.BP_InventoryComponent`))
  (return _success))

(fn `UserConstructionScript`)