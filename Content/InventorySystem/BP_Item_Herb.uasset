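; BP_Item_Herb is an inventory item that heals the player when used.
; Its UseItem override calls the parent version, then casts player character 0 to ThirdPersonCharacter and adds HealthToRecover to CurrentHealth, capped at MaxHealth.
; It then refreshes the character's health bar and returns true; the event graph and construction script add no logic of their own.
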(fn `UseItem`
  (returns (Success :type Boolean))
  (`parent.UseItem`)
  (bind _asthird_person_character (cast `/Game/ThirdPersonCPP/Blueprints/ThirdPersonCharacter` (`GameplayStatics.GetPlayerCharacter` 0)))
  (set `/Game/ThirdPersonCPP/Blueprints/ThirdPersonCharacter.CurrentHealth` (`KismetMathLibrary.Min` (+ (`/Game/ThirdPersonCPP/Blueprints/ThirdPersonCharacter.CurrentHealth` _asthird_person_character) (`self.HealthToRecover`)) (`/Game/ThirdPersonCPP/Blueprints/ThirdPersonCharacter.MaxHealth` _asthird_person_character)) _asthird_person_character)
  (`/Game/ThirdPersonCPP/Blueprints/ThirdPersonCharacter.UpdateHealthBar` _asthird_person_character)
  (return true))

(fn `UserConstructionScript`
  (`parent.UserConstructionScript`))