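; BP_ItemMaster is an inventory item Blueprint, named as the master item, that supports interaction and pickup.
; Its live PickUpItem and Interact graphs only defer to parent implementations.
; Disconnected leftover logic gates quest-item pickup on matching quest objective targets, adds the item to the character's inventory, destroys the actor and notifies quests, but never runs.
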(event `self.PickUpItem`
  (`parent.PickUpItem`))

(fn `Interact`
  (params (Interactor :type "Actor Object Reference"))
  (returns (Success :type Boolean))
  (`parent.Interact` Interactor)
  (return true))

(fn `Interact`
  (returns (Interactor :type "Actor Object Reference"))
  (bind _interactor (`parent.Interact`)))

(fn `UserConstructionScript`)