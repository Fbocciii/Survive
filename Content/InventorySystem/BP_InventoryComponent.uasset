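; Inventory component that holds an array of item slots and opens or closes the inventory window.
; It runs PrepareInventory on BeginPlay and before each window opening.
; ToggleInventory creates the widget bound to itself, anchors it centrally on the player controller's HUD canvas and switches between UI-only and game-only input.
; AddToStack tops up a slot to its max stack size and passes any overflow back through AddToInventory.
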(event `self.ReceiveBeginPlay`
  (`self.PrepareInventory`))

(event `self.ToggleInventory`
  (bind _inventorywindow (`self.InventoryWindow`)
    (:`then`
      (`Widget.RemoveFromParent` _inventorywindow)
      (set `self.InventoryWindow` null)
      (`WidgetBlueprintLibrary.SetInputMode_GameOnly` (`GameplayStatics.GetPlayerController` 0)))
    (:`else`
      (`self.PrepareInventory`)
      (bind _returnvalue (`|CreateWidget` "/Game/InventorySystem/InventoryWindow_BP.InventoryWindow_BP_C" null self))
      (set `self.InventoryWindow` _returnvalue)
      (bind _asbp_my_player_controller (cast `/Game/BP_MyPlayerController` (`GameplayStatics.GetPlayerController` 0)))
      (bind _returnvalue_2 (`CanvasPanel.AddChildToCanvas` (`/Game/InventorySystem/HUD.HudCanvas` (`/Game/BP_MyPlayerController.HUDWidget` _asbp_my_player_controller)) (`self.InventoryWindow`)))
      (`CanvasPanelSlot.SetAutoSize` _returnvalue_2 true)
      (`CanvasPanelSlot.SetAlignment` _returnvalue_2 (0.5 0.5))
      (`CanvasPanelSlot.SetAnchors` _returnvalue_2 (make `Anchors` (0.5 0.5) (0.5 0.5)))
      (`CanvasPanelSlot.SetPosition` _returnvalue_2 (`self.Position`))
      (`WidgetBlueprintLibrary.SetInputMode_UIOnlyEx` _asbp_my_player_controller (`self.InventoryWindow`) "LockAlways"))))

(fn `AddToStack`
  (params (SlotStructure :type "SlotStructure Structure") (SlotIndex :type Integer))
  (returns (Success :type Boolean))
  (locals (CurrentStackQuantity :type Integer))
  (bind (_slotstructure_itemstructure _slotstructure_quantity) (break `SlotStructure` (`local.SlotStructure`)))
  (bind _slotstructure_itemstructure_2 (break `SlotStructure` (`local.SlotStructure`)))
  (bind (_slotstructure_itemstructure_3 _slotstructure_quantity_2) (break `SlotStructure` (`local.SlotStructure`)))
  (bind _inventory (`self.Inventory`))
  (bind (_name _description _thumbnail _maxstacksize) (break `ItemStructure` _slotstructure_itemstructure_2))
  (bind (_output_itemstructure _output_quantity) (break `SlotStructure` (`|GetArrayItem` _inventory (`local.SlotIndex`))))
  (bind (_itemstructure _quantity) (break `SlotStructure` (`|GetArrayItem` (`self.Inventory`) SlotIndex)))
  (bind _output_get (set `local.CurrentStackQuantity` _quantity))
  (if (> (+ _output_get (`.Quantity` (break `SlotStructure` SlotStructure))) (`.MaxStackSize` (break `ItemStructure` _itemstructure)))
    (`KismetArrayLibrary.Array_Set` (`self.Inventory`) (`local.SlotIndex`) (make `SlotStructure` _slotstructure_itemstructure_2 _maxstacksize))
    (`self.AddToInventory` (make `SlotStructure` _slotstructure_itemstructure_3 (- _slotstructure_quantity_2 (- _maxstacksize (`local.CurrentStackQuantity`)))))
    (else
      (`KismetArrayLibrary.Array_Set` _inventory (`local.SlotIndex`) (make `SlotStructure` _output_itemstructure (+ _output_quantity _slotstructure_quantity)))))
  (return true))