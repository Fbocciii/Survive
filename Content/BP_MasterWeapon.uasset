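; Base weapon Blueprint for the third-person character, handling light and heavy melee combo attacks and enemy damage.
; Each attack plays the montage at the character's chain index, flags the last attack, then advances the index with wraparound.
; HitEvent matches the hit actor against all MasterEnemy actors, damages each enemy once via AlreadyDamagedEnemy, and adds 30% for heavy attacks.
; Interact, combo events and AttackTrace are empty stubs.
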(event `/Game/InventorySystem/InteractInterface.Interact`
  (params (Interactor :type "Actor Object Reference")))

(event `self.ReceiveBeginPlay`
  (bind _asthird_person_character (cast `/Game/ThirdPersonCPP/Blueprints/ThirdPersonCharacter` (`GameplayStatics.GetPlayerCharacter` 0)))
  (set `self.CharacterRef` _asthird_person_character))

(event `LightAttack`
  (bind _characterref (`self.CharacterRef`))
  (bind _characterref_2 (`self.CharacterRef`))
  (bind _chainlightattack (`/Game/ThirdPersonCPP/Blueprints/ThirdPersonCharacter.ChainLightAttack` _characterref_2))
  (if (== (+ (`/Game/ThirdPersonCPP/Blueprints/ThirdPersonCharacter.ChainLightAttack` (`self.CharacterRef`)) 1) (`KismetArrayLibrary.Array_Length` (`self.LightAttacks`)))
    (set `/Game/ThirdPersonCPP/Blueprints/ThirdPersonCharacter.LastAttack` true (`self.CharacterRef`)))
  (`Character.PlayAnimMontage` _characterref (`|GetArrayItem` (`self.LightAttacks`) (`/Game/ThirdPersonCPP/Blueprints/ThirdPersonCharacter.ChainLightAttack` _characterref)) 1.0 "None")
  (`self.Combo Light Attack` _chainlightattack)
  (set `/Game/ThirdPersonCPP/Blueprints/ThirdPersonCharacter.ChainLightAttack` (mod (+ _chainlightattack 1) (`KismetArrayLibrary.Array_Length` (`self.LightAttacks`))) _characterref_2))

(event `HeavyAttack`
  (bind _characterref (`self.CharacterRef`))
  (bind _characterref_2 (`self.CharacterRef`))
  (bind _chainheavyattack (`/Game/ThirdPersonCPP/Blueprints/ThirdPersonCharacter.ChainHeavyAttack` _characterref_2))
  (if (== (+ (`/Game/ThirdPersonCPP/Blueprints/ThirdPersonCharacter.ChainHeavyAttack` (`self.CharacterRef`)) 1) (`KismetArrayLibrary.Array_Length` (`self.HeavyAttacks`)))
    (set `/Game/ThirdPersonCPP/Blueprints/ThirdPersonCharacter.LastAttack` true (`self.CharacterRef`)))
  (`Character.PlayAnimMontage` _characterref (`|GetArrayItem` (`self.HeavyAttacks`) (`/Game/ThirdPersonCPP/Blueprints/ThirdPersonCharacter.ChainHeavyAttack` _characterref)) 1.0 "None")
  (`self.Combo Heavy Attack` _chainheavyattack)
  (set `/Game/ThirdPersonCPP/Blueprints/ThirdPersonCharacter.ChainHeavyAttack` (mod (+ _chainheavyattack 1) (`KismetArrayLibrary.Array_Length` (`self.HeavyAttacks`))) _characterref_2))

(event `Combo Light Attack`
  (params (ChainLightAttack :type Integer)))

(event `Combo Heavy Attack`
  (params (ChainHeavyAttack :type Integer)))

(event `HitEvent`
  (params (Damage :type Integer) (Hit :type "HitResult Structure"))
  (bind _characterref (`self.CharacterRef`))
  (set `self.Damage` Damage)
  (bind _outactors (`GameplayStatics.GetAllActorsOfClass` "/Game/ThirdPersonCPP/Blueprints/MasterEnemy.MasterEnemy_C"))
  (for _array_element _outactors
    (set `self.DamagedEnemy` _array_element)
    (if (and (== _array_element (`.HitActor` (`GameplayStatics.BreakHitResult` Hit))) (not (`KismetArrayLibrary.Array_Contains` (`self.AlreadyDamagedEnemy`) (`self.DamagedEnemy`))))
      (`KismetArrayLibrary.Array_Add` (`self.AlreadyDamagedEnemy`) (`self.DamagedEnemy`))
      (if (`/Game/ThirdPersonCPP/Blueprints/ThirdPersonCharacter.LightAttack` _characterref)
        (`/Game/ThirdPersonCPP/Blueprints/HealthDamageInterface.DealingDamage` (`self.DamagedEnemy`) (`self.Damage`) (`self.CharacterRef`))
        (elif (`/Game/ThirdPersonCPP/Blueprints/ThirdPersonCharacter.HeavyAttack` _characterref)
          (`/Game/ThirdPersonCPP/Blueprints/HealthDamageInterface.DealingDamage` (`self.DamagedEnemy`) (+ (`self.Damage`) (`KismetMathLibrary.FTrunc` (* (`self.Damage`) 0.3))) (`self.CharacterRef`)))))))

(fn `AttackTrace`)

(fn `UserConstructionScript`)