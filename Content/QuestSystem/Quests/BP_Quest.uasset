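; Quest actor that tracks a list of objectives for reaching locations, interacting, collecting items and killing enemies.
; On BeginPlay it caches the player's inventory and binds to the four matching gameplay events.
; Location and interaction checks match exact targets; collection and kills match by class, using an inventory query or one shared kill counter.
; Completed objectives refresh the HUD objectives widget, and an editor helper snaps the quest to its parent actor.
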(event `self.ReceiveBeginPlay`
  (bind _asthird_person_character (cast `/Game/ThirdPersonCPP/Blueprints/ThirdPersonCharacter` (`GameplayStatics.GetPlayerCharacter` 0)))
  (set `self.PlayerInventory` (`/Game/ThirdPersonCPP/Blueprints/ThirdPersonCharacter.BP_InventoryComponent` _asthird_person_character))
  (add `self.LocationReached` (`|CreateDelegate` :!event `CheckLocationObjective`))
  (add `self.Interacted` (`|CreateDelegate` :!event `CheckInteractionObjective`))
  (add `self.CollectedItem` (`|CreateDelegate` :!event `CheckCollectionObjective`))
  (add `self.KilledEnemy` (`|CreateDelegate` :!event `CheckKillObjective`)))

(fn `CheckCollectionObjective`
  (params (Item :type "/Game/InventorySystem/BP_ItemMaster Object Reference"))
  (locals (UpdateUI :type Boolean) (ObjectiveNumber :type Integer))
  (bind (_output_description _output_type _output_iscomplete _output_target _output_number) (break `/Game/QuestSystem/Objectives/ObjectiveData_BP` (`|GetArrayItem` (`self.Objectives`) (`local.ObjectiveNumber`))))
  (for (_array_element _array_index) (`self.Objectives`)
    (set `local.ObjectiveNumber` _array_index)
    (bind (_description _type _iscomplete _target _number) (break `/Game/QuestSystem/Objectives/ObjectiveData_BP` _array_element))
    (if (== (`GameplayStatics.GetObjectClass` _target) (`GameplayStatics.GetObjectClass` (`local.Item`)))
      (bind _isininventory (`/Game/InventorySystem/BP_InventoryComponent.InventoryQuery` (`self.PlayerInventory`) (`|MakeArray` (make `InventoryQuery` (`GameplayStatics.GetObjectClass` (`local.Item`)) _number) :!type "InventoryQuery Structure")))
      (if _isininventory
        (`KismetArrayLibrary.Array_Set` (`self.Objectives`) (`local.ObjectiveNumber`) (make `/Game/QuestSystem/Objectives/ObjectiveData_BP` _output_description _output_type true _output_target _output_number))
        (set `local.UpdateUI` true))))
  (if (`local.UpdateUI`)
    (bind _asbp_my_player_controller (cast `/Game/BP_MyPlayerController` (`GameplayStatics.GetPlayerController` 0)))
    (`/Game/QuestSystem/QuestUI/UI_Objectives.UpdateObjectives` (`/Game/InventorySystem/HUD.UI_Objectives` (`/Game/BP_MyPlayerController.HUDWidget` _asbp_my_player_controller)))))

(fn `CheckInteractionObjective`
  (params (InteractionTarget :type "Actor Object Reference"))
  (locals (ObjectiveNumber :type Integer :default 0) (UpdateUI :type Boolean :default true))
  (bind (_output_description _output_type _output_iscomplete _output_target _output_number) (break `/Game/QuestSystem/Objectives/ObjectiveData_BP` (`|GetArrayItem` (`self.Objectives`) (`local.ObjectiveNumber`))))
  (for (_array_element _array_index) (`self.Objectives`)
    (set `local.ObjectiveNumber` _array_index)
    (bind (_description _type _iscomplete _target) (break `/Game/QuestSystem/Objectives/ObjectiveData_BP` _array_element))
    (if (and (not _iscomplete) (== _target (`local.InteractionTarget`)))
      (`KismetArrayLibrary.Array_Set` (`self.Objectives`) (`local.ObjectiveNumber`) (make `/Game/QuestSystem/Objectives/ObjectiveData_BP` _output_description _output_type true _output_target _output_number))
      (set `local.UpdateUI` true)))
  (if (`local.UpdateUI`)
    (bind _asbp_my_player_controller (cast `/Game/BP_MyPlayerController` (`GameplayStatics.GetPlayerController` 0)))
    (`/Game/QuestSystem/QuestUI/UI_Objectives.UpdateObjectives` (`/Game/InventorySystem/HUD.UI_Objectives` (`/Game/BP_MyPlayerController.HUDWidget` _asbp_my_player_controller)))))

(fn `CheckKillObjective`
  (params (Enemy :type "/Game/ThirdPersonCPP/Blueprints/MasterEnemy_OLD Object Reference"))
  (locals (ObjectiveNumber :type Integer) (UpdateUI :type Boolean))
  (bind (_output_description _output_type _output_iscomplete _output_target _output_number) (break `/Game/QuestSystem/Objectives/ObjectiveData_BP` (`|GetArrayItem` (`self.Objectives`) (`local.ObjectiveNumber`))))
  (for (_array_element _array_index) (`self.Objectives`)
    (bind (_description _type _iscomplete _target _number) (break `/Game/QuestSystem/Objectives/ObjectiveData_BP` _array_element))
    (if (== (`GameplayStatics.GetObjectClass` _target) (`GameplayStatics.GetObjectClass` (`local.Enemy`)))
      (set `local.ObjectiveNumber` _array_index)
      (bind _result (`/Engine/EditorBlueprintResources/StandardMacros.IncrementInt` (`self.CurrentKillCount`))
        (:`  `
          (if (>= _result _number)
            (set `local.UpdateUI` true)
            (`KismetArrayLibrary.Array_Set` (`self.Objectives`) (`local.ObjectiveNumber`) (make `/Game/QuestSystem/Objectives/ObjectiveData_BP` _output_description _output_type true _output_target _output_number)))))))
  (if (`local.UpdateUI`)
    (bind _asbp_my_player_controller (cast `/Game/BP_MyPlayerController` (`GameplayStatics.GetPlayerController` 0)))
    (`/Game/QuestSystem/QuestUI/UI_Objectives.UpdateObjectives` (`/Game/InventorySystem/HUD.UI_Objectives` (`/Game/BP_MyPlayerController.HUDWidget` _asbp_my_player_controller)))))

(fn `CheckLocationObjective`
  (params (LocationReached :type "/Game/QuestSystem/BP_LocationMarker Object Reference"))
  (locals (ObjectiveNumber :type Integer) (UpdateUI :type Boolean))
  (bind (_output_description _output_type _output_iscomplete _output_target _output_number) (break `/Game/QuestSystem/Objectives/ObjectiveData_BP` (`|GetArrayItem` (`self.Objectives`) (`local.ObjectiveNumber`))))
  (for (_array_element _array_index) (`self.Objectives`)
    (set `local.ObjectiveNumber` _array_index)
    (bind (_description _type _iscomplete _target) (break `/Game/QuestSystem/Objectives/ObjectiveData_BP` _array_element))
    (if (and (not _iscomplete) (== _target (`local.LocationReached`)))
      (`KismetArrayLibrary.Array_Set` (`self.Objectives`) (`local.ObjectiveNumber`) (make `/Game/QuestSystem/Objectives/ObjectiveData_BP` _output_description _output_type true _output_target _output_number))
      (set `local.UpdateUI` true)))
  (if (`local.UpdateUI`)
    (bind _asbp_my_player_controller (cast `/Game/BP_MyPlayerController` (`GameplayStatics.GetPlayerController` 0)))
    (`/Game/QuestSystem/QuestUI/UI_Objectives.UpdateObjectives` (`/Game/InventorySystem/HUD.UI_Objectives` (`/Game/BP_MyPlayerController.HUDWidget` _asbp_my_player_controller)))))

(fn `OrganizeQuestInEditor`
  (`self.K2_SetActorLocation` (`self.K2_GetActorLocation` (`self.GetAttachParentActor`))))

(fn `UserConstructionScript`)