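; BP_QuestLog manages showing and hiding the quest log UI through a single ToggleQuestLog function.
; Opening creates a UI_QuestLog widget and adds it to the HUD canvas of BP_MyPlayerController, anchored to fill the screen.
; Closing removes the widget, clears its reference and restores game-only input, movement and a hidden cursor.
; The UI-only input and cursor-showing nodes are disconnected, so opening leaves input unchanged.
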(fn `ToggleQuestLog`
  (bind _returnvalue (`GameplayStatics.GetPlayerController` 0))
  (bind _questlogui (`self.QuestLogUI`)
    (:`then`
      (`Widget.RemoveFromParent` _questlogui)
      (set `self.QuestLogUI` null)
      (`WidgetBlueprintLibrary.SetInputMode_GameOnly` _returnvalue)
      (`Controller.SetIgnoreMoveInput` _returnvalue false)
      (set `PlayerController.bShowMouseCursor` false _returnvalue))
    (:`else`
      (bind _returnvalue_2 (`|CreateWidget` "/Game/QuestSystem/QuestUI/UI_QuestLog.UI_QuestLog_C"))
      (set `self.QuestLogUI` _returnvalue_2)
      (bind _asbp_my_player_controller (cast `/Game/BP_MyPlayerController` (`GameplayStatics.GetPlayerController` 0)))
      (bind _returnvalue_3 (`CanvasPanel.AddChildToCanvas` (`/Game/InventorySystem/HUD.HudCanvas` (`/Game/BP_MyPlayerController.HUDWidget` _asbp_my_player_controller)) (`self.QuestLogUI`)))
      (`CanvasPanelSlot.SetAnchors` _returnvalue_3 (make `Anchors` (0.0 0.0) (1.0 1.0))))))