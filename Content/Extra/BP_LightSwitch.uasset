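; Trigger-box light switch that fades the level between day and night as the third-person character enters or leaves.
; Both overlaps share a FlipFlop that plays or reverses a timeline, pitching the sun, updating the sky sphere and dimming sun and skylight within a night pitch range.
; On finish, it either opens a slideshow media source and lights all FairyLight actors one by one via a delayed ForEach macro, or switches them off.
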(event `self.ReceiveBeginPlay`
  (bind _outactors (`GameplayStatics.GetAllActorsOfClass` "/Game/Extra/FairyLight.FairyLight_C"))
  (set `self.LightArray` _outactors))

(event `self.Box.OnComponentBeginOverlap`
  (params (OverlappedComponent :type "PrimitiveComponent Object Reference") (OtherActor :type "Actor Object Reference") (OtherComp :type "PrimitiveComponent Object Reference") (OtherBodyIndex :type Integer) (bFromSweep :type Boolean) (SweepResult :type "HitResult Structure (by ref)"))
  (bind _lightsource (`self.LightSource`))
  (bind (_returnvalue_roll _returnvalue_pitch) (`KismetMathLibrary.BreakRotator` (`self.K2_GetActorRotation` _lightsource)))
  (bind (_returnvalue_roll_2 _returnvalue_pitch_2 _returnvalue_yaw) (`KismetMathLibrary.BreakRotator` (`self.K2_GetActorRotation` _lightsource)))
  (bind _lightcomponent (`Light.LightComponent` (`self.LightSource`)))
  (bind _lightcomponent_2 (`SkyLight.LightComponent` (`self.SkyLight`)))
  (bind _asthird_person_character (cast `/Game/ThirdPersonCPP/Blueprints/ThirdPersonCharacter` OtherActor))
  (if (== (`Character.CapsuleComponent` _asthird_person_character) OtherComp)
    (bind _isa (`/Engine/EditorBlueprintResources/StandardMacros.FlipFlop` :!label _label)
      (:`A`
        (bind (_direction _dim _time) (`Timeline|Timeline_0` :!label _label_2)
          (:`Update`
            (`self.K2_SetActorRotation` _lightsource (`KismetMathLibrary.MakeRotator` _returnvalue_roll_2 _dim _returnvalue_yaw) false)
            (`/Engine/EngineSky/BP_Sky_Sphere.UpdateSunDirection` (`self.SkySphere`))
            (bind _output_get (set `self.NightTime` (`KismetMathLibrary.InRange_FloatFloat` _returnvalue_pitch -30.0 60.0)))
            (if _output_get
              (bind _returnvalue (`KismetMathLibrary.Abs` (- _time (`self.PrevTime`))))
              (`LightComponent.SetIntensity` _lightcomponent (`KismetMathLibrary.FInterpTo` (`LightComponentBase.Intensity` _lightcomponent) 0.1 _returnvalue 1.0))
              (`SkyLightComponent.SetIntensity` _lightcomponent_2 (`KismetMathLibrary.FInterpTo` (`LightComponentBase.Intensity` _lightcomponent_2) 0.01 (/ _returnvalue 4.0) 2.0))
              (set `self.PrevTime` _time)))
          (:`Finished`
            (if _isa
              (`MediaPlayer.OpenSource` (`self.Slideshow`) "/Game/Media/20190824_193712.20190824_193712")
              (bind _arrayelement (`self.ForEachDelay` (`self.LightArray`) 1.0)
                (:`LoopBody`
                  (`/Game/Extra/FairyLight.TurnOn` _arrayelement)))
              (else
                (for _array_element (`self.LightArray`)
                  (`/Game/Extra/FairyLight.TurnOff` _array_element)))))))
      (:`B`
        (goto _label_2 :!via `Reverse`)))))

(event `self.Box.OnComponentEndOverlap`
  (params (OverlappedComponent :type "PrimitiveComponent Object Reference") (OtherActor :type "Actor Object Reference") (OtherComp :type "PrimitiveComponent Object Reference") (OtherBodyIndex :type Integer))
  (bind _asthird_person_character (cast `/Game/ThirdPersonCPP/Blueprints/ThirdPersonCharacter` OtherActor))
  (if (== (`Character.CapsuleComponent` _asthird_person_character) OtherComp)
    (goto _label)))

(fn `UserConstructionScript`)