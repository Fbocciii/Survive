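; Runs a timed fireworks show, started by Interact alongside the opening of the "1Year" media source.
; BeginPlay sorts TS_FireworksLauncher actors into Initial, Finale and Heart groups by actor tag.
; A custom ForEachDelay macro staggers launches and positional sounds: Initial shells first, then after a long pause a rapid finale, then hearts.
; The finale also refires Initial launchers by matching array index after random delays.
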(event `self.ReceiveBeginPlay`
  (bind _outactors (`GameplayStatics.GetAllActorsWithTag` "Initial"))
  (for _array_element _outactors
    (bind _asts_fireworks_launcher (cast `/Game/TS_Fireworks/Blueprints/TS_FireworksLauncher` _array_element))
    (`KismetArrayLibrary.Array_Add` (`self.InitialFireworks`) _asts_fireworks_launcher))
  (bind _outactors_2 (`GameplayStatics.GetAllActorsWithTag` "Finale"))
  (for _array_element_2 _outactors_2
    (bind _asts_fireworks_launcher_2 (cast `/Game/TS_Fireworks/Blueprints/TS_FireworksLauncher` _array_element_2))
    (`KismetArrayLibrary.Array_Add` (`self.FinaleFireworks`) _asts_fireworks_launcher_2))
  (bind _outactors_3 (`GameplayStatics.GetAllActorsWithTag` "Heart"))
  (for _array_element_3 _outactors_3
    (bind _asts_fireworks_launcher_3 (cast `/Game/TS_Fireworks/Blueprints/TS_FireworksLauncher` _array_element_3))
    (`KismetArrayLibrary.Array_Add` (`self.HeartFireworks`) _asts_fireworks_launcher_3)))

(event `BeginFireworks`
  (`MediaPlayer.OpenSource` (`self.1YearShow`) "/Game/Media/1Year.1Year")
  (`KismetSystemLibrary.Delay` 5.0)
  (bind _arrayelement (`self.ForEachDelay` (`self.InitialFireworks`) 4.0)
    (:`LoopBody`
      (`/Game/TS_Fireworks/Blueprints/TS_FireworksLauncher.LaunchShell` _arrayelement)
      (`GameplayStatics.PlaySoundAtLocation` (`self.LaunchSound`) (`self.K2_GetActorLocation` _arrayelement) (struct) 1.0 1.0 0.0 (`self.FireworkAttenuation`) null _arrayelement))
    (:`Completed`
      (`KismetSystemLibrary.Delay` 85.0)
      (bind (_arrayelement_2 _arrayindex) (`self.ForEachDelay` (`self.FinaleFireworks`) 0.25)
        (:`LoopBody`
          (`/Game/TS_Fireworks/Blueprints/TS_FireworksLauncher.LaunchShell` _arrayelement_2)
          (`GameplayStatics.PlaySoundAtLocation` (`self.LaunchSound`) (`self.K2_GetActorLocation` _arrayelement_2) (struct) 0.5 1.0 0.0 (`self.FireworkAttenuation`) null null)
          (`KismetSystemLibrary.Delay` (`KismetMathLibrary.RandomFloatInRange` 0.5 1.5))
          (`/Game/TS_Fireworks/Blueprints/TS_FireworksLauncher.LaunchShell` (`|GetArrayItem` (`self.InitialFireworks`) _arrayindex))
          (`GameplayStatics.PlaySoundAtLocation` (`self.LaunchSound`) (`self.K2_GetActorLocation`) (struct) 0.5 1.0 0.0 (`self.FireworkAttenuation`) null null))
        (:`Completed`
          (bind _arrayelement_3 (`self.ForEachDelay` (`self.HeartFireworks`) (`KismetMathLibrary.RandomFloatInRange` 1.25 2.25))
            (:`LoopBody`
              (`/Game/TS_Fireworks/Blueprints/TS_FireworksLauncher.LaunchShell` _arrayelement_3)
              (`GameplayStatics.PlaySoundAtLocation` (`self.LaunchSound`) (`self.K2_GetActorLocation` _arrayelement_3) (struct) 1.0 1.0 0.0 (`self.FireworkAttenuation`) null null))))))))

(event `/Game/InventorySystem/InteractInterface.Interact`
  (params (Interactor :type "Actor Object Reference"))
  (`self.BeginFireworks`))

(fn `UserConstructionScript`)