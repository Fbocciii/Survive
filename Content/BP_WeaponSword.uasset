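; Sword weapon Blueprint that handles combo chaining and melee hit detection for its owning character.
; Light and heavy combo events each set the character's other chain index, subtracting that attack array's length on overflow so combos can switch type.
; AttackTrace casts short line traces backward from six sphere components against Pawns, ignoring the owner, and passes hits with damage to HitEvent.
; The traces leave debug drawing enabled.
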(event `self.Combo Light Attack`
  (params (ChainLightAttack :type Integer))
  (bind _characterref (`self.CharacterRef`))
  (bind _returnvalue (`KismetArrayLibrary.Array_Length` (`self.HeavyAttacks`)))
  (if (>= ChainLightAttack _returnvalue)
    (set `/Game/ThirdPersonCPP/Blueprints/ThirdPersonCharacter.ChainHeavyAttack` (- ChainLightAttack _returnvalue) _characterref)
    (else
      (set `/Game/ThirdPersonCPP/Blueprints/ThirdPersonCharacter.ChainHeavyAttack` ChainLightAttack _characterref))))

(event `self.Combo Heavy Attack`
  (params (ChainHeavyAttack :type Integer))
  (bind _characterref (`self.CharacterRef`))
  (bind _returnvalue (`KismetArrayLibrary.Array_Length` (`self.LightAttacks`)))
  (if (>= ChainHeavyAttack _returnvalue)
    (set `/Game/ThirdPersonCPP/Blueprints/ThirdPersonCharacter.ChainLightAttack` (- ChainHeavyAttack _returnvalue) _characterref)
    (else
      (set `/Game/ThirdPersonCPP/Blueprints/ThirdPersonCharacter.ChainLightAttack` ChainHeavyAttack _characterref))))

(event `self.AttackTrace`
  (for _array_element (`|MakeArray` (`self.Sphere`) (`self.Sphere1`) (`self.Sphere2`) (`self.Sphere4`) (`self.Sphere5`) (`self.Sphere6`))
    (bind _returnvalue (`SceneComponent.K2_GetComponentLocation` _array_element))
    (bind (_outhit _returnvalue_2) (`KismetSystemLibrary.LineTraceSingleForObjects` _returnvalue (- _returnvalue (* (`KismetMathLibrary.GetForwardVector` (`SceneComponent.K2_GetComponentRotation` _array_element)) 5.0)) (`|MakeArray` "ObjectTypeQuery3" :!type "EObjectTypeQuery Enum") true (`|MakeArray` (`self.CharacterRef`) :!type "Actor Object Reference") "ForDuration" true (struct :`R` 1.0 :`A` 1.0) (struct :`G` 1.0 :`A` 1.0) 0.2))
    (if _returnvalue_2
      (`self.HitEvent` (`self.Damage`) _outhit))))

(fn `UserConstructionScript`
  (`parent.UserConstructionScript`))